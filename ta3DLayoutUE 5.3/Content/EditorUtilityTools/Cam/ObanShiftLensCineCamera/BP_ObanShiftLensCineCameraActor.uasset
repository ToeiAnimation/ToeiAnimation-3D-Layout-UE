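; Shift-lens cine camera actor for "Oban" (large-format) layouts, displaying up to five toggleable frame guide meshes in front of the camera.
; FrameOffset sits at a set camera distance, scaled from FOV and standard-to-render width ratio, updating on construction, distance change or ChangeFrameEvent.
; Construction creates per-frame dynamic materials for color and edge/fill style.
; Helpers validate and correct frame transforms to in-plane offset, roll and uniform scale.
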(event `self.ReceiveBeginPlay`)

(event `self.ReceiveTick`
  (params (DeltaSeconds :type "Float (single-precision)")))

(event `UpdateFrameOffsetTransformEvent`
  ;[1 1 1] FrameOffsetのTransformを更新
  (`self.UpdateFrameOffsetTransform`))

(event `ChangeFrameEvent`
  (params (RenderResolutionWidth :type Integer))
  ;[1 1 1] Frame変更時イベント
  (set `self.RenderResolutionWidth` RenderResolutionWidth)
  (`self.UpdateFrameOffsetTransformEvent`))

(fn `Calc Frame Offset Size`
  (returns (FrameSize :type "Vector Structure"))
  (locals (StandardFrameWidth :type "Float (double-precision)" :default 2000.0))
  (bind _returnvalue (* (* (* (`KismetMathLibrary.DegTan` (/ (`CameraComponent.FieldOfView` (`self.CameraComponent`)) 2.0)) (`self.DistanceCameraToFrame`)) 2.0) (/ (`local.StandardFrameWidth`) (`self.RenderResolutionWidth`))))
  ;[1 1 1] FOVからフレームサイズ取得
  (return (`KismetMathLibrary.MakeVector` _returnvalue _returnvalue _returnvalue)) ; 長さ=フレームのサイズとなるため算出した値をVectorにして返す
)

(fn `CorrectInvalid TransformFrame`
  (params (index :type Integer))
  (bind _smframe (`self.GetSmFrame` index))
  (bind (_relativelocation_x _relativelocation_y _relativelocation_z) (`KismetMathLibrary.BreakVector` (`SceneComponent.RelativeLocation` _smframe)))
  ;[1 1 1] 不正なトランスフォーム値を更新(Pos.X,Rot.Y,Zは常に0, ScaleはXYZが均等)
  (`SceneComponent.K2_SetRelativeLocation` _smframe (`KismetMathLibrary.MakeVector` 0.0 _relativelocation_y _relativelocation_z) false false)
  (bind _relativerotation_roll (`KismetMathLibrary.BreakRotator` (`SceneComponent.RelativeRotation` _smframe)))
  (`SceneComponent.K2_SetRelativeRotation` _smframe (`KismetMathLibrary.MakeRotator` _relativerotation_roll) false false)
  (bind (_relativescale3d_x _relativescale3d_y) (`KismetMathLibrary.BreakVector` (`SceneComponent.RelativeScale3D` _smframe)))
  (`SceneComponent.SetRelativeScale3D` _smframe (`KismetMathLibrary.MakeVector` _relativescale3d_y _relativescale3d_y _relativescale3d_y)))

(fn `GetDistanceCameraToFrame`
  (returns (value :type "Float (double-precision)"))
  (return (`self.DistanceCameraToFrame`)))

(fn `GetEnable`
  (params (index :type Integer))
  (returns (Enable :type Boolean))
  (switch `int` index
    (:`Default`
      (`KismetSystemLibrary.PrintString` "An unexpected index is specified"))
    (:`0`
      (return (`self.Enable0`)))
    (:`1`
      (return (`self.Enable1`)))
    (:`2`
      (return (`self.Enable2`)))
    (:`3`
      (return (`self.Enable3`)))
    (:`4`
      (return (`self.Enable4`)))))

(fn `GetFrameMaterialInstance`
  (params (index :type Integer))
  (returns (NewParam :type "MaterialInstanceDynamic Object Reference"))
  (bind _materialinstance0 (`self.MaterialInstance0`))
  (bind _materialinstance1 (`self.MaterialInstance1`))
  (bind _materialinstance2 (`self.MaterialInstance2`))
  (bind _materialinstance3 (`self.MaterialInstance3`))
  (bind _materialinstance4 (`self.MaterialInstance4`))
  (switch `int` index
    (:`0`
      (`/Engine/EditorBlueprintResources/StandardMacros.IsValid` _materialinstance0
        (:`Is Valid`
          (return _materialinstance0))
        (:`Is Not Valid`
          _)))
    (:`1`
      (`/Engine/EditorBlueprintResources/StandardMacros.IsValid` _materialinstance1
        (:`Is Valid`
          (return _materialinstance1))
        (:`Is Not Valid`
          _)))
    (:`2`
      (`/Engine/EditorBlueprintResources/StandardMacros.IsValid` _materialinstance2
        (:`Is Valid`
          (return _materialinstance2))
        (:`Is Not Valid`
          _)))
    (:`3`
      (`/Engine/EditorBlueprintResources/StandardMacros.IsValid` _materialinstance3
        (:`Is Valid`
          (return _materialinstance3))
        (:`Is Not Valid`
          _)))
    (:`4`
      (`/Engine/EditorBlueprintResources/StandardMacros.IsValid` _materialinstance4
        (:`Is Valid`
          (return _materialinstance4))
        (:`Is Not Valid`
          _))))
  (`KismetSystemLibrary.PrintString` "Material Instance が取得できませんでした"))

(fn `GetFrameMaterialInstanceArray`
  (returns (materialInstances :type "Array of MaterialInstanceDynamic Object Reference"))
  (return (`|MakeArray` (`self.MaterialInstance0`) (`self.MaterialInstance1`) (`self.MaterialInstance2`) (`self.MaterialInstance3`) (`self.MaterialInstance4`))))

(fn `GetSmFrame`
  (params (index :type Integer))
  (returns (SmFrame :type "StaticMeshComponent Object Reference"))
  (switch `int` index
    (:`Default`
      (`KismetSystemLibrary.PrintString` "An unexpected index is specified"))
    (:`0`
      (return (`self.SM_FrameA`)))
    (:`1`
      (return (`self.SM_FrameB`)))
    (:`2`
      (return (`self.SM_FrameC`)))
    (:`3`
      (return (`self.SM_FrameD`)))
    (:`4`
      (return (`self.SM_FrameE`)))))

(fn `Init`
  (`self.InitFrameMaterialInstance`))

(fn `InitFrameMaterialInstance`
  (`|ExecutionSequence`
    (:`then_0`
      (`/Engine/EditorBlueprintResources/StandardMacros.IsValid` (`self.MaterialInstance0`)
        (:`Is Not Valid`
          (bind _returnvalue (`PrimitiveComponent.CreateDynamicMaterialInstance` (`self.SM_FrameA`) 0 "/Game/EditorUtilityTools/Cam/ObanShiftLensCineCamera/M_ObanFrame.M_ObanFrame" "None"))
          (set `self.MaterialInstance0` _returnvalue))))
    (:`then_1`
      (`/Engine/EditorBlueprintResources/StandardMacros.IsValid` (`self.MaterialInstance1`)
        (:`Is Not Valid`
          (bind _returnvalue_2 (`PrimitiveComponent.CreateDynamicMaterialInstance` (`self.SM_FrameB`) 0 "/Game/EditorUtilityTools/Cam/ObanShiftLensCineCamera/M_ObanFrame.M_ObanFrame" "None"))
          (set `self.MaterialInstance1` _returnvalue_2))))
    (:`then_2`
      (`/Engine/EditorBlueprintResources/StandardMacros.IsValid` (`self.MaterialInstance2`)
        (:`Is Not Valid`
          (bind _returnvalue_3 (`PrimitiveComponent.CreateDynamicMaterialInstance` (`self.SM_FrameC`) 0 "/Game/EditorUtilityTools/Cam/ObanShiftLensCineCamera/M_ObanFrame.M_ObanFrame" "None"))
          (set `self.MaterialInstance2` _returnvalue_3))))
    (:`then_3`
      (`/Engine/EditorBlueprintResources/StandardMacros.IsValid` (`self.MaterialInstance3`)
        (:`Is Not Valid`
          (bind _returnvalue_4 (`PrimitiveComponent.CreateDynamicMaterialInstance` (`self.SM_FrameD`) 0 "/Game/EditorUtilityTools/Cam/ObanShiftLensCineCamera/M_ObanFrame.M_ObanFrame" "None"))
          (set `self.MaterialInstance3` _returnvalue_4))))
    (:`then_4`
      (`/Engine/EditorBlueprintResources/StandardMacros.IsValid` (`self.MaterialInstance4`)
        (:`Is Not Valid`
          (bind _returnvalue_5 (`PrimitiveComponent.CreateDynamicMaterialInstance` (`self.SM_FrameE`) 0 "/Game/EditorUtilityTools/Cam/ObanShiftLensCineCamera/M_ObanFrame.M_ObanFrame" "None"))
          (set `self.MaterialInstance4` _returnvalue_5))))))

(fn `MakeValidationMessage`
  (params (object :type "Object Object Reference") (message :type String))
  (returns (return :type String))
  (return (`KismetStringLibrary.Concat_StrStr` (`KismetSystemLibrary.GetDisplayName` (`ActorComponent.GetOwner` (`self.RootComponent`))) " / " (`KismetSystemLibrary.GetObjectName` object) " >> " message)))

(fn `SetDistanceCameraToFrame`
  (params (value :type "Float (double-precision)"))
  (set `self.DistanceCameraToFrame` value)
  (`self.UpdateFrameOffsetTransform`) ; 値の変更に伴いフレームオフセットの更新を行う
)

(fn `SetEnable`
  (params (index :type Integer) (value :type Boolean))
  (switch `int` index
    (:`Default`
      (`KismetSystemLibrary.PrintString` "An unexpected index is specified"))
    (:`0`
      (set `self.Enable0` value))
    (:`1`
      (set `self.Enable1` value))
    (:`2`
      (set `self.Enable2` value))
    (:`3`
      (set `self.Enable3` value))
    (:`4`
      (set `self.Enable4` value))))

(fn `SetEnableAndReferencePropertyUpdate`
  (params (index :type Integer) (value :type Boolean))
  (`self.SetEnable` index value)
  (`self.ValidateEnableAndUpdateVisible` index) ; Enableの評価とVisibilityの更新
)

(fn `SetFrameStyle`
  (params (FrameStyle :type "/Game/EditorUtilityTools/Cam/ObanShiftLensCineCamera/EBP_ObanFrameStyle Enum" :default "NewEnumerator0"))
  (bind _output_get (set `self.FrameStyle` FrameStyle))
  (`self.SetMaterialParameterFrameStyle` _output_get))

(fn `SetMaterialParameterFrameColor`
  (params (index :type Integer) (value :type "Color Structure"))
  (bind _newparam (`self.GetFrameMaterialInstance` index))
  (`MaterialInstanceDynamic.SetVectorParameterValue` _newparam "Color" (`KismetMathLibrary.Conv_ColorToLinearColor` value)) ; カラー
)

(fn `SetMaterialParameterFrameStyle`
  (params (A :type "/Game/EditorUtilityTools/Cam/ObanShiftLensCineCamera/EBP_ObanFrameStyle Enum" :default "NewEnumerator0"))
  (bind _materialinstances (`self.GetFrameMaterialInstanceArray`))
  (for _array_element _materialinstances
    (switch `/Game/EditorUtilityTools/Cam/ObanShiftLensCineCamera/EBP_ObanFrameStyle` A
      (:`NewEnumerator0`
        (`MaterialInstanceDynamic.SetScalarParameterValue` _array_element "EdgeNo" 1.0)
        (`MaterialInstanceDynamic.SetScalarParameterValue` _array_element "IsEdge" 1.0 :!label _label))
      (:`NewEnumerator2`
        (`MaterialInstanceDynamic.SetScalarParameterValue` _array_element "EdgeNo" 2.0)
        (goto _label))
      (:`NewEnumerator1`
        (`MaterialInstanceDynamic.SetScalarParameterValue` _array_element "IsEdge" 0.0)))))

(fn `SetMaterialParameters`
  ;[1 1 1] FrameStyleの変更
  (`self.SetMaterialParameterFrameStyle` (`self.FrameStyle`))
  ;[1 1 1] フレームカラー変更
  (`self.SetMaterialParameterFrameColor` 0 (`self.FrameColor0`))
  (`self.SetMaterialParameterFrameColor` 1 (`self.FrameColor1`))
  (`self.SetMaterialParameterFrameColor` 2 (`self.FrameColor2`))
  (`self.SetMaterialParameterFrameColor` 3 (`self.FrameColor3`))
  (`self.SetMaterialParameterFrameColor` 4 (`self.FrameColor4`)))

(fn `SetVisibleAllFrame`
  (params (value :type Boolean))
  (`|ExecutionSequence`
    (:`then_0`
      (`self.SetVisibleAndReferencePropertyUpdate` 0 value))
    (:`then_1`
      (`self.SetVisibleAndReferencePropertyUpdate` 1 value))
    (:`then_2`
      (`self.SetVisibleAndReferencePropertyUpdate` 2 value))
    (:`then_3`
      (`self.SetVisibleAndReferencePropertyUpdate` 3 value))
    (:`then_4`
      (`self.SetVisibleAndReferencePropertyUpdate` 4 value))))

(fn `SetVisibleAndReferencePropertyUpdate`
  (params (index :type Integer) (value :type Boolean))
  (bind _smframe (`self.GetSmFrame` index))
  (`SceneComponent.SetVisibility` _smframe value value)
  (bind _enable (`self.GetEnable` index)) ; FrameのEnableを取得
  ;[1 1 1] Enable=Falseの場合は常に非表示
  (if (not _enable)
    (`SceneComponent.SetVisibility` _smframe false false)))

(fn `UpdateFrameOffsetTransform`
  (bind _framesize (`self.Calc Frame Offset Size`)) ; FOV/カメラからフレームまでの距離を元にフレームのサイズを算出する
  (`SceneComponent.K2_SetRelativeTransform` (`self.FrameOffset`) (`KismetMathLibrary.MakeTransform` (`KismetMathLibrary.MakeVector` (`self.DistanceCameraToFrame`)) (struct) _framesize) false false))

(fn `UserConstructionScript`
  (`self.Init`)
  ;[1 1 1] FrameOffsetのTransform更新
  (`self.UpdateFrameOffsetTransform`)
  ;[1 1 1] マテリアルパラメータの更新
  (`self.SetMaterialParameters`))

(fn `ValidateEnableAndUpdateVisible`
  (params (index :type Integer))
  ;[1 1 1] Enable値の評価とVisibleの更新
  (bind _smframe (`self.GetSmFrame` index))
  (bind _enable (`self.GetEnable` index))
  (if _enable
    (`SceneComponent.SetVisibility` _smframe true true)
    (else
      (`SceneComponent.SetVisibility` _smframe false false))))

(fn `ValidateTransformFrame`
  (params (index :type Integer))
  (returns (IsValid :type Boolean) (validationMessages :type "Array of String"))
  (locals (ValidationResultMessages :type "Array of String"))
  (bind _validationresultmessages (`local.ValidationResultMessages`))
  (bind _smframe (`self.GetSmFrame` index))
  (`|ExecutionSequence`
    (:`then_0`
      (bind _return (`self.EqualCustom` (.x (.location (`SceneComponent.GetRelativeTransform` _smframe)))))
      (if (not _return)
        (bind _return_2 (`self.MakeValidationMessage` _smframe "Pos.Xが0ではない"))
        (`KismetArrayLibrary.Array_Add` _validationresultmessages _return_2)))
    (:`then_1`
      (bind _return_3 (`self.EqualCustom` (.pitch (.rotation (`SceneComponent.GetRelativeTransform` _smframe)))))
      (if (not _return_3)
        (bind _return_4 (`self.MakeValidationMessage` _smframe "Rot.Yが0ではない"))
        (`KismetArrayLibrary.Array_Add` _validationresultmessages _return_4)))
    (:`then_2`
      (bind _return_5 (`self.EqualCustom` (.yaw (.rotation (`SceneComponent.GetRelativeTransform` _smframe)))))
      (if (not _return_5)
        (bind _return_6 (`self.MakeValidationMessage` _smframe "Rot.Zが0ではない"))
        (`KismetArrayLibrary.Array_Add` _validationresultmessages _return_6)))
    (:`then_3`
      (bind _returnvalue (and (== (.x (.scale (`SceneComponent.GetRelativeTransform` _smframe))) (.y (.scale (`SceneComponent.GetRelativeTransform` _smframe)))) (== (.y (.scale (`SceneComponent.GetRelativeTransform` _smframe))) (.z (.scale (`SceneComponent.GetRelativeTransform` _smframe))))))
      (if (not _returnvalue)
        (bind _return_7 (`self.MakeValidationMessage` _smframe "Scaleが均一ではない"))
        (`KismetArrayLibrary.Array_Add` _validationresultmessages _return_7)))
    (:`then_4`
      (return (and _return _return_3 _return_5 _returnvalue) _validationresultmessages))))

(fn `ValidateTransformFrameAll`
  (returns (ValidationResultMessages :type "Array of String") (IsValid :type Boolean))
  (locals (ValidationMessages :type "Array of String"))
  (bind _validationmessages (`local.ValidationMessages`))
  (bind (_isvalid _validationmessages_2) (`self.ValidateTransformFrame` 0))
  (`KismetArrayLibrary.Array_Append` _validationmessages _validationmessages_2)
  (bind (_isvalid_2 _validationmessages_3) (`self.ValidateTransformFrame` 1))
  (`KismetArrayLibrary.Array_Append` _validationmessages _validationmessages_3)
  (bind (_isvalid_3 _validationmessages_4) (`self.ValidateTransformFrame` 2))
  (`KismetArrayLibrary.Array_Append` _validationmessages _validationmessages_4)
  (bind (_isvalid_4 _validationmessages_5) (`self.ValidateTransformFrame` 3))
  (`KismetArrayLibrary.Array_Append` _validationmessages _validationmessages_5)
  (bind (_isvalid_5 _validationmessages_6) (`self.ValidateTransformFrame` 4))
  (`KismetArrayLibrary.Array_Append` _validationmessages _validationmessages_6)
  (return (`local.ValidationMessages`) (and _isvalid _isvalid_2 _isvalid_3 _isvalid_4 _isvalid_5)))