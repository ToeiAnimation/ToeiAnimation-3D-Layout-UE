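; BP_DekPlus is a clickable posed-figure actor for a layout editor, with adjustable pose, height, overlay color and visibility.
; Clicking clears other list-linked highlights, highlights this actor and its list entry, and registers it with LayoutMenu and W_ObjectEditor widgets.
; Setters store and apply changes: pose updates both main and highlight meshes, while height becomes uniform actor scale.
; A global visibility toggle respects individual visibility, and Tick caches the transform.
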(event `self.ReceiveBeginPlay`
  (set `self.BP_DekPlus` self))

(event `self.ReceiveTick`
  (params (DeltaSeconds :type "Float (single-precision)"))
  (set `self.Transform` (`self.GetTransform`)))

(event `self.ReceiveActorOnClicked`
  (params (ButtonPressed :type "Key Structure"))
  ;[0 0 0 1 40] クリックで選択状態にする
  (bind _foundwidgets (`WidgetBlueprintLibrary.GetAllWidgetsOfClass` "/Game/PackageKit/Widgets/W_ItemActorList.W_ItemActorList_C" false))
  (for _array_element _foundwidgets
    (`Widget.SetVisibility` (`/Game/PackageKit/Widgets/W_ItemActorList.Border_Active` _array_element) "Collapsed")
    (bind _bp_dekplus (`/Game/PackageKit/Widgets/W_ItemActorList.BP_Dekplus` _array_element)
      (:`then`
        (`SceneComponent.SetVisibility` (`/Game/PackageKit/Blueprints/BP_DekPlus.Mesh_HighLight` _bp_dekplus) false false))
      (:`else`
        _))
    (bind _foundwidgets_2 (`WidgetBlueprintLibrary.GetAllWidgetsOfClass` "/Game/PackageKit/Widgets/LayoutMenu.LayoutMenu_C" false))
    (for _array_element_2 _foundwidgets_2
      (set `/Game/PackageKit/Widgets/LayoutMenu.ActiveW_ActorList` (`self.W_ActorList`) _array_element_2)
      (set `/Game/PackageKit/Widgets/LayoutMenu.BP_DekPlus` self _array_element_2)
      (`/Game/PackageKit/Widgets/LayoutMenu.SetVisbleDekEdit` _array_element_2 "Visible")
      (`SceneComponent.SetVisibility` (`self.Mesh_HighLight`) true false)
      (`Widget.SetVisibility` (`/Game/PackageKit/Widgets/W_ItemActorList.Border_Active` (`self.W_ActorList`)) "HitTestInvisible")
      (bind _foundwidgets_3 (`WidgetBlueprintLibrary.GetAllWidgetsOfClass` "/Game/PackageKit/Widgets/W_ObjectEditor.W_ObjectEditor_C" false))
      (for _array_element_3 _foundwidgets_3
        (set `/Game/PackageKit/Widgets/W_ObjectEditor.BP_DekPlus` self _array_element_3)))))

(event `SetAllVisble`
  (params (Condition :type Boolean))
  (if Condition
    (`SceneComponent.SetVisibility` (`self.Mesh`) (`self.IsVisible`) false)
    (else
      (`SceneComponent.SetVisibility` (`self.Mesh`) false false))))

(event `SetVisible`
  (params (IsVisible :type Boolean))
  (bind _output_get (set `self.IsVisible` IsVisible))
  (`SceneComponent.SetVisibility` (`self.Mesh`) _output_get false))

(event `SetColor`
  (params (NewOverlayMaterial :type "MaterialInterface Object Reference"))
  ;[0 0 0] 色の設定
  (`MeshComponent.SetOverlayMaterial` (`self.Mesh`) NewOverlayMaterial)
  (set `self.OverlayMaterial` NewOverlayMaterial))

(event `SetHeight`
  (params (DekHeight :type "Float (double-precision)"))
  ;[0 0 0] 身長の設定
  (bind _output_get (set `self.DekHeight` DekHeight))
  (`self.SetActorScale3D` (`KismetMathLibrary.Conv_DoubleToVector` (`KismetMathLibrary.SafeDivide` _output_get 100.0))) ; 身長の更新
)

(event `SetPose`
  (params (pose :type "StaticMesh Object Reference") (AssetName :type Text))
  ;[0 0 0] メッシュの設定
  (bind _output_get (set `self.pose` pose))
  (`StaticMeshComponent.SetStaticMesh` (`self.Mesh`) _output_get)
  (`StaticMeshComponent.SetStaticMesh` (`self.Mesh_HighLight`) _output_get)
  (set `self.AssetName` AssetName))

(fn `UserConstructionScript`)